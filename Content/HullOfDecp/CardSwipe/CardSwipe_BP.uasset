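; CardSwipe_BP is a card swipe task object that gives text feedback and shows success on its indicator lights.
; The player entering its box briefly shows a ShowTextInterface widget, removed early on exit.
; StartOperation calls OP, defined outside these graphs, unless the task is completed.
; TooFast and TooSlow flash timed warning widgets, while Won switches material brightness from the red light to the green.
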(event OnComponentBeginOverlap(Box)
  (params (OverlappedComponent :type Primitive%20Component%20Object%20Reference) (OtherActor :type Actor%20Object%20Reference) (OtherComp :type Primitive%20Component%20Object%20Reference) (OtherBodyIndex :type Integer) (bFromSweep :type Boolean) (SweepResult :type Hit%20Result%20Structure%20%28by%20ref%29))
  ;[1 1 1] Begin/End Overlap Operations
  (if (== OtherActor (Game|GetPlayerCharacter 0))
    (bind _returnvalue (UserInterface|CreateWidget "/Game/HullOfDecp/ShowTextInterface.ShowTextInterface_C" (Game|GetPlayerController 0)))
    (UserInterface|Viewport|AddtoViewport _returnvalue 0)
    (Utilities|FlowControl|Delay 3.0)
    (Widget|RemovefromParent _returnvalue)))

(event OnComponentEndOverlap(Box)
  (params (OverlappedComponent :type Primitive%20Component%20Object%20Reference) (OtherActor :type Actor%20Object%20Reference) (OtherComp :type Primitive%20Component%20Object%20Reference) (OtherBodyIndex :type Integer))
  ;[1 1 1] Begin/End Overlap Operations
  (Utilities|IsValid (stale OnComponentBeginOverlap(Box) _returnvalue)
    (:Is%20Valid
      (Widget|RemovefromParent (stale OnComponentBeginOverlap(Box) _returnvalue)))))

(event EventBeginPlay
  (Variables|Default|SetCardMesh (Variables|Default|GetCard)))

(event EventTooFast
  (bind _returnvalue (UserInterface|CreateWidget "/Game/HullOfDecp/ShowTextInterface.ShowTextInterface_C"))
  (Variables|/Game/HullOfDecp/ShowTextInterface.ShowTextInterface_C|SetTextToShow _returnvalue "Too Fast........")
  (UserInterface|Viewport|AddtoViewport _returnvalue 0)
  (Utilities|FlowControl|Delay 1.0)
  (Widget|RemovefromParent _returnvalue))

(event EventTooSlow
  (bind _returnvalue (UserInterface|CreateWidget "/Game/HullOfDecp/ShowTextInterface.ShowTextInterface_C"))
  (Variables|/Game/HullOfDecp/ShowTextInterface.ShowTextInterface_C|SetTextToShow _returnvalue "Too Slow........")
  (UserInterface|Viewport|AddtoViewport _returnvalue 0)
  (Utilities|FlowControl|Delay 1.0)
  (Widget|RemovefromParent _returnvalue))

(event EventStartOperation
  (if (not (Variables|Default|GetIsCompleted))
    (Class|CardSwipe|OP)))

(event EventWon
  (Rendering|Material|SetScalarParameterValueonMaterials (Variables|Default|GetGreenLight) "Brighness" 5e+01)
  (Rendering|Material|SetScalarParameterValueonMaterials (Variables|Default|GetRedLight) "Brighness" 0.0))

(fn ConstructionScript)