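; Interactable radio that opens an adjustment widget for the player, with an animated material on its right screen.
; An AI character entering its box changes the screen's tiling and speed and marks it completed, while other characters get a text prompt removed after three seconds or on exit.
; StartOperation, if not completed, calls OP and hands the screen and itself to a RadioAdjustWidget.
; A separate event reveals the radio icon sprite.
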(event OnComponentBeginOverlap(BoxCollision)
  (params (OverlappedComponent :type Primitive%20Component%20Object%20Reference) (OtherActor :type Actor%20Object%20Reference) (OtherComp :type Primitive%20Component%20Object%20Reference) (OtherBodyIndex :type Integer) (bFromSweep :type Boolean) (SweepResult :type Hit%20Result%20Structure%20%28by%20ref%29))
  (bind _rightscreen (Variables|Default|GetRightScreen))
  (bind _ashulls_of_deception_character (Utilities|Casting|CastToHullsOfDeceptionCharacter OtherActor))
  (if (Variables|/Script/HullsOfDeception.HullsOfDeceptionCharacter|GetIsAI _ashulls_of_deception_character)
    (Rendering|Material|SetScalarParameterValueonMaterials _rightscreen "UTiling" 0.2)
    (Rendering|Material|SetVectorParameterValueonMaterials _rightscreen "Speed" (Math|Vector|MakeVector 1.0 0.0 0.0))
    (Variables|Default|SetIsCompleted true)
    (else
      (bind _returnvalue (UserInterface|CreateWidget "/Game/HullOfDecp/ShowTextInterface.ShowTextInterface_C" (Game|GetPlayerController 0)))
      (UserInterface|Viewport|AddtoViewport _returnvalue 0)
      (Utilities|FlowControl|Delay 3.0)
      (Widget|RemovefromParent _returnvalue))))

(event OnComponentEndOverlap(BoxCollision)
  (params (OverlappedComponent :type Primitive%20Component%20Object%20Reference) (OtherActor :type Actor%20Object%20Reference) (OtherComp :type Primitive%20Component%20Object%20Reference) (OtherBodyIndex :type Integer))
  (Utilities|IsValid (stale OnComponentBeginOverlap(BoxCollision) _returnvalue)
    (:Is%20Valid
      (Widget|RemovefromParent (stale OnComponentBeginOverlap(BoxCollision) _returnvalue)))))

(event EventBeginPlay
  (bind _rightscreen (Variables|Default|GetRightScreen))
  (Variables|Default|SetLeftScreen (Variables|Default|GetLeftScreenBP))
  (Rendering|Material|SetScalarParameterValueonMaterials _rightscreen "UTiling" 0.8)
  (Rendering|Material|SetVectorParameterValueonMaterials _rightscreen "Speed" "5.000000, 0, 0")
  (Rendering|Material|SetVectorParameterValueonMaterials _rightscreen "Color" "0.141643,1.000000, 0"))

(event EventStartOperation
  (if (not (Variables|Default|GetIsCompleted))
    (Class|Radio|OP)
    (bind _returnvalue (UserInterface|CreateWidget "/Game/HullOfDecp/Radio/RadioAdjustWidget.RadioAdjustWidget_C" (Game|GetPlayerController 0)))
    (UserInterface|Viewport|AddtoViewport _returnvalue 0)
    (Variables|/Game/HullOfDecp/Radio/RadioAdjustWidget.RadioAdjustWidget_C|SetRadioObject _returnvalue (Variables|Default|GetRightScreen))
    (Variables|/Game/HullOfDecp/Radio/RadioAdjustWidget.RadioAdjustWidget_C|SetRadioObjectRef _returnvalue self)))

(event EventSpriteEnableDisable
  (Development|SetHiddeninGame (Variables|Default|GetRadioICON_Sprite) false false))

(fn ConstructionScript)