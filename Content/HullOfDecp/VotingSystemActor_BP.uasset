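; Voting actor that runs an emergency meeting when a body is found, in an Among Us-style imposter game.
; FoundDead runs once, freezing input, opening MeetingWidget and casting random votes among living characters into its per-color tallies.
; Votesollected? kills the top-voted color's character (TaskDivider_BP's list, or the player for White).
; It then briefly shows whether that was an Imposter, restores input and destroys dead characters.
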(event Custom|GenerateRandomVotes
  (bind _out_actors_0 (Variables|Default|GetOut%20Actors_0))
  (for _index (range 0 (- (Utilities|Array|Length _out_actors_0) 1))
    (CallFunction|CollectVotes (Variables|/Game/ThirdPersonCPP/Blueprints/ThirdPersonCharacter.ThirdPersonCharacter_C|GetNumber (.OutItem (Utilities|Array|Random _out_actors_0))))
    (Variables|Default|SetVoteNo (+ (Variables|Default|GetVoteNo) 1))))

(event Custom|Collect%20Votes
  (params (NewParam :type Integer))
  (bind _meetingwidget (Variables|Default|GetMeetingWidget))
  (bind _meetingwidget_2 (Variables|Default|GetMeetingWidget))
  (bind _meetingwidget_3 (Variables|Default|GetMeetingWidget))
  (bind _meetingwidget_4 (Variables|Default|GetMeetingWidget))
  (bind _meetingwidget_5 (Variables|Default|GetMeetingWidget))
  (bind _meetingwidget_6 (Variables|Default|GetMeetingWidget))
  (switch int NewParam
    (:1
      (Variables|/Game/HullOfDecp/MeetingWidget/MeetingWidget.MeetingWidget_C|SetYellow _meetingwidget (+ (Variables|/Game/HullOfDecp/MeetingWidget/MeetingWidget.MeetingWidget_C|GetYellow _meetingwidget) 1)))
    (:2
      (Variables|/Game/HullOfDecp/MeetingWidget/MeetingWidget.MeetingWidget_C|SetGreen _meetingwidget_5 (+ 1 (Variables|/Game/HullOfDecp/MeetingWidget/MeetingWidget.MeetingWidget_C|GetGreen _meetingwidget_5))))
    (:3
      (Variables|/Game/HullOfDecp/MeetingWidget/MeetingWidget.MeetingWidget_C|SetBlue _meetingwidget_4 (+ 1 (Variables|/Game/HullOfDecp/MeetingWidget/MeetingWidget.MeetingWidget_C|GetBlue _meetingwidget_4))))
    (:4
      (Variables|/Game/HullOfDecp/MeetingWidget/MeetingWidget.MeetingWidget_C|SetBrown _meetingwidget_2 (+ 1 (Variables|/Game/HullOfDecp/MeetingWidget/MeetingWidget.MeetingWidget_C|GetBrown _meetingwidget_2))))
    (:5
      (Variables|/Game/HullOfDecp/MeetingWidget/MeetingWidget.MeetingWidget_C|SetRed _meetingwidget_6 (+ (Variables|/Game/HullOfDecp/MeetingWidget/MeetingWidget.MeetingWidget_C|GetRed _meetingwidget_6) 1)))
    (:6
      (Variables|/Game/HullOfDecp/MeetingWidget/MeetingWidget.MeetingWidget_C|SetWhite _meetingwidget_3 (+ 1 (Variables|/Game/HullOfDecp/MeetingWidget/MeetingWidget.MeetingWidget_C|GetWhite _meetingwidget_3))))))

(event Custom|Votesollected?
  (bind _meetingwidget (Variables|Default|GetMeetingWidget))
  (Widget|RemovefromParent (Variables|Default|GetMeetingWidget))
  (bind _outactors (Actor|GetAllActorsOfClass "/Game/TaskDivider_BP.TaskDivider_BP_C"))
  (switch int (.IndexOfMaxValue (Math|Integer|MaxOfIntArray (Utilities|Array|MakeArray (Variables|/Game/HullOfDecp/MeetingWidget/MeetingWidget.MeetingWidget_C|GetYellow _meetingwidget) (Variables|/Game/HullOfDecp/MeetingWidget/MeetingWidget.MeetingWidget_C|GetGreen _meetingwidget) (Variables|/Game/HullOfDecp/MeetingWidget/MeetingWidget.MeetingWidget_C|GetBlue _meetingwidget) (Variables|/Game/HullOfDecp/MeetingWidget/MeetingWidget.MeetingWidget_C|GetBrown _meetingwidget) (Variables|/Game/HullOfDecp/MeetingWidget/MeetingWidget.MeetingWidget_C|GetRed _meetingwidget) (Variables|/Game/HullOfDecp/MeetingWidget/MeetingWidget.MeetingWidget_C|GetWhite _meetingwidget))))
    (:0
      (Class|DeathInterface|Die (Utilities|Array|Get(acopy) (Variables|/Script/HullsOfDeception.TaskDivider|GetCharacters (Utilities|Array|Get(acopy) _outactors))))
      (if (Variables|/Script/HullsOfDeception.HullsOfDeceptionCharacter|GetIsImposter (Utilities|Array|Get(acopy) (Variables|/Script/HullsOfDeception.TaskDivider|GetCharacters (Utilities|Array|Get(acopy) _outactors))))
        (bind _returnvalue (UserInterface|CreateWidget "/Game/HullOfDecp/ShowTextInterface.ShowTextInterface_C" :!label _label))
        (Variables|/Game/HullOfDecp/ShowTextInterface.ShowTextInterface_C|SetTextToShow _returnvalue "That one was Imposter")
        (UserInterface|Viewport|AddtoViewport _returnvalue 0)
        (Utilities|FlowControl|Delay 4.0)
        (Widget|RemovefromParent _returnvalue)
        (else
          (bind _returnvalue_2 (UserInterface|CreateWidget "/Game/HullOfDecp/ShowTextInterface.ShowTextInterface_C" :!label _label_2))
          (Variables|/Game/HullOfDecp/ShowTextInterface.ShowTextInterface_C|SetTextToShow _returnvalue_2 "That one was not Imposter")
          (UserInterface|Viewport|AddtoViewport _returnvalue_2 0)
          (Utilities|FlowControl|Delay 4.0)
          (Widget|RemovefromParent _returnvalue_2))))
    (:1
      (Class|DeathInterface|Die (Utilities|Array|Get(acopy) (Variables|/Script/HullsOfDeception.TaskDivider|GetCharacters (Utilities|Array|Get(acopy) _outactors)) 1))
      (if (Variables|/Script/HullsOfDeception.HullsOfDeceptionCharacter|GetIsImposter (Utilities|Array|Get(acopy) (Variables|/Script/HullsOfDeception.TaskDivider|GetCharacters (Utilities|Array|Get(acopy) _outactors)) 1))
        (goto _label)
        (else
          (goto _label_2))))
    (:2
      (Class|DeathInterface|Die (Utilities|Array|Get(acopy) (Variables|/Script/HullsOfDeception.TaskDivider|GetCharacters (Utilities|Array|Get(acopy) _outactors)) 2))
      (if (Variables|/Script/HullsOfDeception.HullsOfDeceptionCharacter|GetIsImposter (Utilities|Array|Get(acopy) (Variables|/Script/HullsOfDeception.TaskDivider|GetCharacters (Utilities|Array|Get(acopy) _outactors)) 2))
        (goto _label)
        (else
          (goto _label_2))))
    (:3
      (Class|DeathInterface|Die (Utilities|Array|Get(acopy) (Variables|/Script/HullsOfDeception.TaskDivider|GetCharacters (Utilities|Array|Get(acopy) _outactors)) 3))
      (if (Variables|/Script/HullsOfDeception.HullsOfDeceptionCharacter|GetIsImposter (Utilities|Array|Get(acopy) (Variables|/Script/HullsOfDeception.TaskDivider|GetCharacters (Utilities|Array|Get(acopy) _outactors)) 3))
        (goto _label)
        (else
          (goto _label_2))))
    (:4
      (Class|DeathInterface|Die (Utilities|Array|Get(acopy) (Variables|/Script/HullsOfDeception.TaskDivider|GetCharacters (Utilities|Array|Get(acopy) _outactors)) 4))
      (if (Variables|/Script/HullsOfDeception.HullsOfDeceptionCharacter|GetIsImposter (Utilities|Array|Get(acopy) (Variables|/Script/HullsOfDeception.TaskDivider|GetCharacters (Utilities|Array|Get(acopy) _outactors)) 4))
        (goto _label)
        (else
          (goto _label_2))))
    (:5
      (bind _asthird_person_character (Utilities|Casting|CastToThirdPersonCharacter (Game|GetPlayerCharacter 0)))
      (Class|DeathInterface|Die _asthird_person_character)
      (if (Variables|/Script/HullsOfDeception.HullsOfDeceptionCharacter|GetIsImposter _asthird_person_character)
        (goto _label)
        (else
          (goto _label_2)))))
  (for _array_element (Variables|Default|GetOut%20Actors_0)
    (Input|EnableInput _array_element 0))
  (Variables|/Script/Engine.PlayerController|SetbShowMouseCursor (Game|GetPlayerController 0) false)
  (bind _outactors_2 (Actor|GetAllActorsOfClass "/Game/ThirdPersonCPP/Blueprints/ThirdPersonCharacter.ThirdPersonCharacter_C"))
  (for _array_element_2 _outactors_2
    (if (Variables|/Script/HullsOfDeception.HullsOfDeceptionCharacter|GetIsDead _array_element_2)
      (Actor|DestroyActor _array_element_2))))

(event EventBeginPlay)

(event Collision|EventActorBeginOverlap
  (params (OtherActor :type Actor%20Object%20Reference)))

(event EventFoundDead
  (Utilities|FlowControl|DoOnce false
    (:Completed
      (bind _outactors (Actor|GetAllActorsOfClass "/Game/ThirdPersonCPP/Blueprints/ThirdPersonCharacter.ThirdPersonCharacter_C"))
      (bind _output_get (Variables|Default|SetOut%20Actors_0 _outactors))
      (for _array_element _output_get
        (if (Variables|/Script/HullsOfDeception.HullsOfDeceptionCharacter|GetIsDead _array_element)
          (Utilities|Array|RemoveItem (Variables|Default|GetOut%20Actors_0) _array_element)
          (else
            (Input|DisableInput _array_element (Game|GetPlayerController 0)))))
      (Variables|/Script/Engine.PlayerController|SetbShowMouseCursor (Game|GetPlayerController 0) true)
      (bind _returnvalue (UserInterface|CreateWidget "/Game/HullOfDecp/MeetingWidget/MeetingWidget.MeetingWidget_C" (Game|GetPlayerController 0)))
      (bind _output_get_2 (Variables|Default|SetMeetingWidget _returnvalue))
      (UserInterface|Viewport|AddtoViewport _returnvalue 0)
      (CallFunction|GenerateRandomVotes))))

(event EventTick
  (params (DeltaSeconds :type Float%20%28single-precision%29)))

(fn ConstructionScript)