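; A wire task station that can be sabotaged once while CanSabotage is set, revealing its wire icon sprite.
; BeginPlay caches four colored wire ends and attachments, and StartOperation calls OP until the task is completed.
; Its collision box flags overlapping characters as interacting: AI instantly snaps the wire ends into place and completes the task.
; The local player instead gets a text prompt widget, removed after a delay or on leaving.
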(event OnComponentBeginOverlap(CollisionBox)
  (params (OverlappedComponent :type Primitive%20Component%20Object%20Reference) (OtherActor :type Actor%20Object%20Reference) (OtherComp :type Primitive%20Component%20Object%20Reference) (OtherBodyIndex :type Integer) (bFromSweep :type Boolean) (SweepResult :type Hit%20Result%20Structure%20%28by%20ref%29))
  (bind _ashulls_of_deception_character (Utilities|Casting|CastToHullsOfDeceptionCharacter OtherActor))
  (Variables|/Script/HullsOfDeception.HullsOfDeceptionCharacter|SetIsInteracting _ashulls_of_deception_character true)
  (if (Variables|/Script/HullsOfDeception.HullsOfDeceptionCharacter|GetIsAI _ashulls_of_deception_character)
    (Transformation|SetRelativeLocation (Variables|Default|GetBrownEnd) "21.464600,3.875000,18.759001" false false)
    (Transformation|SetRelativeLocation (Variables|Default|GetBlueEnd) "21.421000,3.875500,15.459000" false false)
    (Transformation|SetRelativeLocation (Variables|Default|GetRedEnd) "21.398800,3.875500,22.792000" false false)
    (Transformation|SetRelativeLocation (Variables|Default|GetGreenEnd) "21.368000,3.855000,11.119000" false false)
    (Variables|Default|SetIsCompleted true)
    (elif (== OtherActor (Game|GetPlayerCharacter 0))
      (bind _returnvalue (UserInterface|CreateWidget "/Game/HullOfDecp/ShowTextInterface.ShowTextInterface_C" (Game|GetPlayerController 0)))
      (UserInterface|Viewport|AddtoViewport _returnvalue 0)
      (Utilities|FlowControl|Delay 3.0)
      (Widget|RemovefromParent _returnvalue))))

(event OnComponentEndOverlap(CollisionBox)
  (params (OverlappedComponent :type Primitive%20Component%20Object%20Reference) (OtherActor :type Actor%20Object%20Reference) (OtherComp :type Primitive%20Component%20Object%20Reference) (OtherBodyIndex :type Integer))
  (bind _ashulls_of_deception_character (Utilities|Casting|CastToHullsOfDeceptionCharacter OtherActor))
  (Variables|/Script/HullsOfDeception.HullsOfDeceptionCharacter|SetIsInteracting _ashulls_of_deception_character false)
  (Utilities|IsValid (stale OnComponentBeginOverlap(CollisionBox) _returnvalue)
    (:Is%20Valid
      (Widget|RemovefromParent (stale OnComponentBeginOverlap(CollisionBox) _returnvalue)))))

(event Custom|Sabotag
  (if (Variables|Default|GetCanSabotage)
    (Class|WireSystem|Sabotage)
    (Variables|Default|SetCanSabotage false)
    (Development|SetHiddeninGame (Variables|Default|GetWireICON_Sprite) false false)))

(event EventBeginPlay
  (Variables|Default|SetBrownWire (Variables|Default|GetBrownEnd))
  (Variables|Default|SetGreenWire (Variables|Default|GetGreenEnd))
  (Variables|Default|SetRedWire (Variables|Default|GetRedEnd))
  (Variables|Default|SetBlueWire (Variables|Default|GetBlueEnd))
  (Variables|Default|SetBrownAttachment (Variables|Default|GetBrownAttachment1))
  (Variables|Default|SetGreenAttachment (Variables|Default|GetGreenAttachment1))
  (Variables|Default|SetRedAttachment (Variables|Default|GetRedAttachment1))
  (Variables|Default|SetBlueAttachment (Variables|Default|GetBlueAttachment1)))

(event EventStartOperation
  (if (not (Variables|Default|GetIsCompleted))
    (Class|WireSystem|OP)))

(event EventSpriteEnableDisable
  (Development|SetHiddeninGame (Variables|Default|GetWireICON_Sprite) false false))

(fn ConstructionScript)