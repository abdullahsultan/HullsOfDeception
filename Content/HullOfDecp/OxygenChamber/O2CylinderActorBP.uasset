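; Oxygen cylinder task station, a Blueprint over a C++ base that receives its collision box at BeginPlay.
; Overlapping characters are flagged as interacting; AI instantly fills O2 and completes the task, while the local player gets a prompt widget for up to three seconds.
; StartOperation opens the O2 progress widget linked to this cylinder, shows the cursor and disables player input.
; SpriteEnableDisable only unhides the Paper sprite.
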(event OnComponentBeginOverlap(BoxCollisionBP)
  (params (OverlappedComponent :type Primitive%20Component%20Object%20Reference) (OtherActor :type Actor%20Object%20Reference) (OtherComp :type Primitive%20Component%20Object%20Reference) (OtherBodyIndex :type Integer) (bFromSweep :type Boolean) (SweepResult :type Hit%20Result%20Structure%20%28by%20ref%29))
  ;[1 1 1] Begin/End Overlap Operations
  (bind _ashulls_of_deception_character (Utilities|Casting|CastToHullsOfDeceptionCharacter OtherActor))
  (Variables|/Script/HullsOfDeception.HullsOfDeceptionCharacter|SetIsInteracting _ashulls_of_deception_character true)
  (if (Variables|/Script/HullsOfDeception.HullsOfDeceptionCharacter|GetIsAI _ashulls_of_deception_character)
    (Variables|Default|SetO2 1e+02)
    (Variables|Default|SetIsCompleted true)
    (elif (== OtherActor (Game|GetPlayerCharacter 0))
      (bind _returnvalue (UserInterface|CreateWidget "/Game/HullOfDecp/ShowTextInterface.ShowTextInterface_C"))
      (UserInterface|Viewport|AddtoViewport _returnvalue 0)
      (Utilities|FlowControl|Delay 3.0)
      (Widget|RemovefromParent _returnvalue))))

(event OnComponentEndOverlap(BoxCollisionBP)
  (params (OverlappedComponent :type Primitive%20Component%20Object%20Reference) (OtherActor :type Actor%20Object%20Reference) (OtherComp :type Primitive%20Component%20Object%20Reference) (OtherBodyIndex :type Integer))
  ;[1 1 1] Begin/End Overlap Operations
  (bind _ashulls_of_deception_character (Utilities|Casting|CastToHullsOfDeceptionCharacter OtherActor))
  (Variables|/Script/HullsOfDeception.HullsOfDeceptionCharacter|SetIsInteracting _ashulls_of_deception_character false)
  (Utilities|IsValid (stale OnComponentBeginOverlap(BoxCollisionBP) _returnvalue)
    (:Is%20Valid
      (Widget|RemovefromParent (stale OnComponentBeginOverlap(BoxCollisionBP) _returnvalue)))))

(event EventBeginPlay
  ;[1 1 1] Sending refrence to C++ variable
  (Variables|Default|SetBoxCollision (Variables|Default|GetBoxCollisionBP)))

(event EventStartOperation
  (bind _returnvalue (Game|GetPlayerController 0))
  ;[1 1 1] Start Operation
  (bind _returnvalue_2 (UserInterface|CreateWidget "/Game/HullOfDecp/OxygenChamber/O2ProgressWidget.O2ProgressWidget_C" _returnvalue))
  (Variables|/Game/HullOfDecp/OxygenChamber/O2ProgressWidget.O2ProgressWidget_C|SetO2CylinderObject _returnvalue_2 self)
  (UserInterface|Viewport|AddtoViewport _returnvalue_2 0)
  (Variables|/Script/Engine.PlayerController|SetbShowMouseCursor _returnvalue true)
  (Input|DisableInput (Game|GetPlayerCharacter 0) _returnvalue))

(event EventSpriteEnableDisable
  (Development|SetHiddeninGame (Variables|Default|GetPaperSprite) false false))

(fn ConstructionScript)